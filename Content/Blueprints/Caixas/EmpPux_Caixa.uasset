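; EmpPux_Caixa is a box that the Personagem1 character picks up by touching it and releases with the Q key.
; On overlap it enables input, sets EstaNaArea and attaches its PaperSprite to the character's capsule.
; Releasing Q clears the flag, detaches the sprite and sweeps it to the player's location.
; End overlap also enables input rather than disabling it, so Q stays bound outside the area.
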(event Collision|EventActorBeginOverlap
  (params (OtherActor :type Actor%20Object%20Reference))
  ;[1 1 1] Evento Pegar Caixa
  (Utilities|Casting|CastToPersonagem1 OtherActor)
  (Input|EnableInput (Game|GetPlayerController 0))
  (Variables|Default|SetEstaNaArea true)
  (bind _aspersonagem_1 (Utilities|Casting|CastToPersonagem1 (Game|GetPlayerCharacter 0)))
  (if (Variables|Default|GetEstaNaArea)
    (Transformation|AttachComponentToComponent (Variables|Components|GetPaperSprite) (Variables|/Script/Engine.Character|GetCapsuleComponent _aspersonagem_1) "None" "KeepWorld" "KeepRelative" "KeepRelative" true)))

(event Collision|EventActorEndOverlap
  (params (OtherActor :type Actor%20Object%20Reference))
  ;[1 1 1] Evento Pegar Caixa
  (Utilities|Casting|CastToPersonagem1 OtherActor)
  (Input|EnableInput (Game|GetPlayerController 0)))

(event Input|KeyboardEvents|Q
  (params (Key :type Key%20Structure))
  (bind _returnvalue (Game|GetPlayerCharacter 0))
  ;[1 1 1] Comando Q: Soltar a Caixa
  (:Released
    (Utilities|Casting|CastToPersonagem1 _returnvalue)
    (Variables|Default|SetEstaNaArea false)
    (Transformation|DetachFromComponent (Variables|Components|GetPaperSprite) "KeepWorld" "KeepWorld" "KeepWorld" true)
    (Transformation|SetWorldLocation (Variables|Components|GetPaperSprite) (Transformation|GetActorLocation _returnvalue) true false)))

(fn ConstructionScript)
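; ElectrodeJumpscare is a sprite-and-capsule box actor that Personagem1 can drop; despite the name, the file shows no jumpscare logic.
; Both begin and end overlap with Personagem1 enable input, so it is never disabled here.
; Releasing Q detaches PaperSprite and Capsule and sweeps them to the player's location.
; The pickup logic attaching both to the player's capsule is unconnected and never runs.
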(event Collision|EventActorBeginOverlap
  (params (OtherActor :type Actor%20Object%20Reference))
  ;[1 1 1] Evento Pegar Caixa
  (Utilities|Casting|CastToPersonagem1 OtherActor)
  (Input|EnableInput (Game|GetPlayerController 0)))

(event Collision|EventActorEndOverlap
  (params (OtherActor :type Actor%20Object%20Reference))
  ;[1 1 1] Evento Pegar Caixa
  (Utilities|Casting|CastToPersonagem1 OtherActor)
  (Input|EnableInput (Game|GetPlayerController 0)))

(event Input|KeyboardEvents|Q
  (params (Key :type Key%20Structure))
  (bind _returnvalue (Game|GetPlayerCharacter 0))
  ;[1 1 1] Comando Q: Soltar a Caixa
  (:Released
    (Utilities|Casting|CastToPersonagem1 _returnvalue)
    (Transformation|DetachFromComponent (Variables|Components|GetPaperSprite) "KeepWorld" "KeepWorld" "KeepWorld" false)
    (Transformation|SetWorldLocation (Variables|Components|GetPaperSprite) (Transformation|GetActorLocation _returnvalue) true false)
    (Transformation|DetachFromComponent (Variables|Components|GetCapsule) "KeepWorld" "KeepWorld" "KeepWorld" false)
    (Transformation|SetWorldLocation (Variables|Components|GetCapsule) (Transformation|GetActorLocation (Game|GetPlayerCharacter 0)) true false)))

(fn ConstructionScript)
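; Sign actor that teaches the player how to read signs, showing the TutorialLerPlacas widget while E is held.
; Overlap by Personagem1 enables input on the actor and briefly flashes a "hold E" prompt widget; leaving disables input.
; Pressing E sets TaLendoPlaca on the character, opens the tutorial and clears the prompt.
; Releasing E removes the tutorial if that flag is set, without resetting it here.
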(event EventBeginPlay)

(event Collision|EventActorBeginOverlap
  (params (OtherActor :type Actor%20Object%20Reference))
  (Utilities|Casting|CastToPersonagem1 OtherActor)
  (Input|EnableInput (Game|GetPlayerController 0))
  (bind _returnvalue (UserInterface|CreateWidget "/Game/Widgets/Tutorials/SegureE.SegureE_C"))
  (UserInterface|Viewport|AddtoViewport _returnvalue 0)
  (Utilities|FlowControl|Delay 0.4)
  (Widget|RemovefromParent _returnvalue))

(event EventTick
  (params (DeltaSeconds :type Float%20%28single-precision%29)))

(event Collision|EventActorEndOverlap
  (params (OtherActor :type Actor%20Object%20Reference))
  (Utilities|Casting|CastToPersonagem1 OtherActor)
  (Input|DisableInput (Game|GetPlayerController 0)))

(event Input|KeyboardEvents|E
  (params (Key :type Key%20Structure))
  (bind _returnvalue (Game|GetPlayerCharacter 0))
  (:Pressed
    (bind _aspersonagem_1 (Utilities|Casting|CastToPersonagem1 _returnvalue))
    (Variables|/Game/Personagem/Personagem1.Personagem1_C|SetTaLendoPlaca _aspersonagem_1 true)
    (Utilities|FlowControl|Sequence
      (:then_0
        (bind _returnvalue_2 (UserInterface|CreateWidget "/Game/Widgets/Tutorials/TutorialLerPlacas.TutorialLerPlacas_C"))
        (UserInterface|Viewport|AddtoViewport _returnvalue_2 0))
      (:then_1
        (Widget|RemovefromParent (stale Collision|EventActorBeginOverlap _returnvalue)))))
  (:Released
    (bind _aspersonagem_1_2 (Utilities|Casting|CastToPersonagem1 _returnvalue))
    (if (Variables|/Game/Personagem/Personagem1.Personagem1_C|GetTaLendoPlaca _aspersonagem_1_2)
      (Widget|RemovefromParent _returnvalue_2))))

(fn ConstructionScript)
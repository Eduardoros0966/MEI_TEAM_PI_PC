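; Blocker actor that moves out of the way for a timed period when the player's first switch is on.
; BeginPlay saves its starting location, and Tick polls the LigouSwitch1 flag on the Personagem1 player character.
; While the flag is set, it teleports to a fixed world position, then after a short Delay returns to the saved location and clears the flag.
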(event EventBeginPlay
  (Variables|Default|SetLocalizacao02 (Transformation|GetActorLocation)))

(event EventTick
  (params (DeltaSeconds :type Float%20%28single-precision%29))
  (bind _aspersonagem_1 (Utilities|Casting|CastToPersonagem1 (Game|GetPlayerCharacter 0)))
  (if (Variables|/Game/Personagem/Personagem1.Personagem1_C|GetLigouSwitch1 _aspersonagem_1)
    (Transformation|SetActorLocation "0,-500.000000, 0" false false)
    (Utilities|FlowControl|Delay 4.5)
    (Transformation|SetActorLocation (Variables|Default|GetLocalizacao02) false false)
    (Variables|/Game/Personagem/Personagem1.Personagem1_C|SetLigouSwitch1 _aspersonagem_1 false)))

(fn ConstructionScript)
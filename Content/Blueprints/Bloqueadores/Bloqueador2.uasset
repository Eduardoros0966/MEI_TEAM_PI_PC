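; Key-locked blocker actor that the player removes with E once Personagem1 holds the first key (PegouChave1).
; On overlap it checks that flag, then either enables input and briefly shows the UsarChave prompt, or briefly shows PrecisaChave.
; Pressing E rechecks the flag, destroys the blocker and removes the prompt.
; Input is never disabled, so E keeps working after the player leaves the overlap.
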(event Collision|EventActorBeginOverlap
  (params (OtherActor :type Actor%20Object%20Reference))
  (bind _aspersonagem_1 (Utilities|Casting|CastToPersonagem1 OtherActor))
  (if (Variables|/Game/Personagem/Personagem1.Personagem1_C|GetPegouChave1 _aspersonagem_1)
    (Input|EnableInput (Game|GetPlayerController 0))
    (Utilities|Casting|CastToPersonagem1 (Game|GetPlayerCharacter 0))
    (bind _returnvalue (UserInterface|CreateWidget "/Game/Widgets/Bloqueadores/UsarChave.UsarChave_C"))
    (UserInterface|Viewport|AddtoViewport _returnvalue 0)
    (Utilities|FlowControl|Delay 0.5)
    (Widget|RemovefromParent _returnvalue)
    (else
      (bind _returnvalue_2 (UserInterface|CreateWidget "/Game/Widgets/Bloqueadores/PrecisaChave.PrecisaChave_C"))
      (UserInterface|Viewport|AddtoViewport _returnvalue_2 0)
      (Utilities|FlowControl|Delay 0.5)
      (Widget|RemovefromParent _returnvalue_2))))

(event EventTick
  (params (DeltaSeconds :type Float%20%28single-precision%29)))

(event Input|KeyboardEvents|E
  (params (Key :type Key%20Structure))
  (:Pressed
    (bind _aspersonagem_1 (Utilities|Casting|CastToPersonagem1 (Game|GetPlayerCharacter 0)))
    (if (Variables|/Game/Personagem/Personagem1.Personagem1_C|GetPegouChave1 _aspersonagem_1)
      (Actor|DestroyActor)
      (Widget|RemovefromParent (stale Collision|EventActorBeginOverlap _returnvalue)))))

(fn ConstructionScript)
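; Blocker actor that moves out of its spot when the player character (Personagem1) has placed box 2, as flagged by ColocouCaixa2.
; BeginPlay stores the starting location.
; Tick polls the flag and, while true, teleports the actor to a fixed world position each frame.
; A three-second Delay then restores the start location; the flag is never cleared here, so the move repeats while it stays set.
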(event EventBeginPlay
  (Variables|Default|SetLocalizacao04 (Transformation|GetActorLocation)))

(event Collision|EventActorBeginOverlap
  (params (OtherActor :type Actor%20Object%20Reference)))

(event EventTick
  (params (DeltaSeconds :type Float%20%28single-precision%29))
  (bind _aspersonagem_1 (Utilities|Casting|CastToPersonagem1 (Game|GetPlayerCharacter 0)))
  (if (Variables|/Game/Personagem/Personagem1.Personagem1_C|GetColocouCaixa2 _aspersonagem_1)
    (Transformation|SetActorLocation "0,-500.000000, 0" false false)
    (Utilities|FlowControl|Delay 3.0)
    (Transformation|SetActorLocation (Variables|Default|GetLocalizacao04) false false)))

(fn ConstructionScript)
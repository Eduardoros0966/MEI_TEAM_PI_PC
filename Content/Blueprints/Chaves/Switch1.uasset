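; Switch1 is an interactable Paper2D switch that the player character, Personagem1, turns on with the E key.
; Actor overlap enables input while Personagem1 is in range and disables it when the overlap ends.
; Pressing E swaps the sprite to Switch2 and sets LigouSwitch1 on the character, so the switch state is recorded on the player.
; The graph has no path to switch it back off.
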(event EventBeginPlay)

(event Collision|EventActorBeginOverlap
  (params (OtherActor :type Actor%20Object%20Reference))
  (Utilities|Casting|CastToPersonagem1 OtherActor)
  (Input|EnableInput (Game|GetPlayerController 0)))

(event EventTick
  (params (DeltaSeconds :type Float%20%28single-precision%29)))

(event Collision|EventActorEndOverlap
  (params (OtherActor :type Actor%20Object%20Reference))
  (Utilities|Casting|CastToPersonagem1 OtherActor)
  (Input|DisableInput (Game|GetPlayerController 0)))

(event Input|KeyboardEvents|E
  (params (Key :type Key%20Structure))
  (:Pressed
    (bind _aspersonagem_1 (Utilities|Casting|CastToPersonagem1 (Game|GetPlayerCharacter 0)))
    (Rendering|Components|Sprite|SetSprite (Variables|Default|GetPaperSprite) "/Game/Sprites/Miscellaneous/Switch2.Switch2")
    (Variables|/Game/Personagem/Personagem1.Personagem1_C|SetLigouSwitch1 _aspersonagem_1 true)))

(fn ConstructionScript)
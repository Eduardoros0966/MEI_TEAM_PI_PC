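; Chave1 is a key pickup actor that the Personagem1 player character collects by pressing E while overlapping it.
; Beginning overlap enables the actor's input and shows an AperteE prompt widget for one second, and ending overlap disables input.
; Pressing E destroys the actor, sets PegouChave1 on the character and removes the prompt from the screen.
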(event EventBeginPlay)

(event Collision|EventActorBeginOverlap
  (params (OtherActor :type Actor%20Object%20Reference))
  (Utilities|Casting|CastToPersonagem1 OtherActor)
  (Utilities|FlowControl|Sequence
    (:then_0
      (Input|EnableInput (Game|GetPlayerController 0)))
    (:then_1
      (bind _returnvalue (UserInterface|CreateWidget "/Game/Widgets/Tutorials/AperteE.AperteE_C"))
      (UserInterface|Viewport|AddtoViewport _returnvalue 0)
      (Utilities|FlowControl|Delay 1.0)
      (Widget|RemovefromParent _returnvalue))))

(event EventTick
  (params (DeltaSeconds :type Float%20%28single-precision%29)))

(event Collision|EventActorEndOverlap
  (params (OtherActor :type Actor%20Object%20Reference))
  (Utilities|Casting|CastToPersonagem1 OtherActor)
  (Input|DisableInput (Game|GetPlayerController 0)))

(event Input|KeyboardEvents|E
  (params (Key :type Key%20Structure))
  (:Pressed
    (bind _aspersonagem_1 (Utilities|Casting|CastToPersonagem1 (Game|GetPlayerCharacter 0)))
    (Actor|DestroyActor)
    (Variables|/Game/Personagem/Personagem1.Personagem1_C|SetPegouChave1 _aspersonagem_1 true)
    (Widget|RemovefromParent (stale Collision|EventActorBeginOverlap _returnvalue))))

(fn ConstructionScript)
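; A counter actor that displays components 1, 2 and 3 in turn once the player places a box, then destroys itself.
; Tick polls the ColocouCaixa flag on the Personagem1 player character and drives a chain of one-second Delays.
; Sequence nodes hide each earlier number as the next appears.
; Tick keeps re-entering the chain while the flag holds, so earlier stages can fire again.
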(event EventBeginPlay)

(event Collision|EventActorBeginOverlap
  (params (OtherActor :type Actor%20Object%20Reference)))

(event EventTick
  (params (DeltaSeconds :type Float%20%28single-precision%29))
  (bind _1 (Variables|Default|Get1))
  (bind _2 (Variables|Default|Get2))
  (bind _aspersonagem_1 (Utilities|Casting|CastToPersonagem1 (Game|GetPlayerCharacter 0)))
  (if (Variables|/Game/Personagem/Personagem1.Personagem1_C|GetColocouCaixa _aspersonagem_1)
    (Utilities|FlowControl|Delay 1.0)
    (Rendering|SetVisibility _1 true false)
    (Utilities|FlowControl|Delay 1.0)
    (Utilities|FlowControl|Sequence
      (:then_0
        (Rendering|SetVisibility _2 true false)
        (Utilities|FlowControl|Delay 1.0)
        (Utilities|FlowControl|Sequence
          (:then_0
            (Rendering|SetVisibility (Variables|Default|Get3) true false)
            (Utilities|FlowControl|Delay 1.0)
            (Actor|DestroyActor))
          (:then_1
            (Rendering|SetVisibility _2 false false))))
      (:then_1
        (Rendering|SetVisibility _1 false false)))))

(fn ConstructionScript)